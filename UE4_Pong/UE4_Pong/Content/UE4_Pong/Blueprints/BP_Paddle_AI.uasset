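; AI-controlled paddle for a Pong game that follows the ball along the X axis.
; Each tick it finds every BP_Gameball and pushes the physics paddle mesh toward it with an impulse from the clamped X offset times AIPaddleSpeed.
; A boundary check then snaps the paddle back to fixed left and right X limits and zeroes its velocity.
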(event `self.ReceiveTick`
  (params (DeltaSeconds :type "Float (single-precision)"))
  ;[1 1 1] Move
  (bind _outactors (`GameplayStatics.GetAllActorsOfClass` "/Game/UE4_Pong/Blueprints/BP_Gameball.BP_Gameball_C"))
  (for _array_element _outactors
    (`PrimitiveComponent.AddImpulse` (`self.SM_Paddle`) (* (`KismetMathLibrary.MakeVector` (`KismetMathLibrary.FClamp` (- (.x (`self.K2_GetActorLocation` _array_element)) (.x (`self.K2_GetActorLocation`))) -2.5 2.5)) (`self.AI_PaddleSpeed`)) "None" false)
    ;[1 1 1] Boundry Check
    (if (> (.x (`self.K2_GetActorLocation`)) 1475.0)
      (`self.K2_SetActorLocation` (`KismetMathLibrary.MakeVector` 1475.0 (.y (`self.K2_GetActorLocation`)) (.z (`self.K2_GetActorLocation`))))
      (`PrimitiveComponent.SetPhysicsLinearVelocity` (`self.SM_Paddle`) (0.0 0.0 0.0) false "None")
      (elif (< (.x (`self.K2_GetActorLocation`)) -1475.0)
        (`self.K2_SetActorLocation` (`KismetMathLibrary.MakeVector` -1475.0 (.y (`self.K2_GetActorLocation`)) (.z (`self.K2_GetActorLocation`))))
        (`PrimitiveComponent.SetPhysicsLinearVelocity` (`self.SM_Paddle`) (0.0 0.0 0.0) false "None")))))

(fn `UserConstructionScript`)