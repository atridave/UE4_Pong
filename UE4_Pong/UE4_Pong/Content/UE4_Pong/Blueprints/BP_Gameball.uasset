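; Pong ball actor that launches along Y, bounces off paddles and boundaries, and keeps the player and CPU scores.
; Overlap casts pick the response: paddles flip Y velocity and pass on their own X velocity, while boundaries flip X.
; Goals increment a score, then a shared path updates the player paddle's score texts and re-serves from the origin toward negative Y.
; The game quits once either score exceeds two.
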(event `self.ReceiveBeginPlay`
  (`PrimitiveComponent.SetPhysicsLinearVelocity` (`self.StaticMeshComponent`) (0.0 -1000.0 0.0) false "None"))

(event `self.ReceiveActorBeginOverlap`
  (params (OtherActor :type "Actor Object Reference"))
  (bind _staticmeshcomponent (`self.StaticMeshComponent`))
  (bind _staticmeshcomponent_2 (`self.StaticMeshComponent`))
  (bind _asbp_paddle_p_1 (cast `/Game/UE4_Pong/Blueprints/BP_Paddle_p1` OtherActor)
    (:`then`
      (bind _returnvalue (`PrimitiveComponent.GetPhysicsLinearVelocity` (`/Game/UE4_Pong/Blueprints/BP_Paddle_p1.SM_Paddle` _asbp_paddle_p_1) "None"))
      (`KismetSystemLibrary.PrintString` "Hit" true true (struct :`G` 1.0 :`B` 0.061501 :`A` 1.0))
      (bind _returnvalue_2 (`PrimitiveComponent.GetPhysicsLinearVelocity` _staticmeshcomponent "None"))
      (`PrimitiveComponent.SetPhysicsLinearVelocity` _staticmeshcomponent (`KismetMathLibrary.MakeVector` (.x _returnvalue) (* (.y _returnvalue_2) -1.0) (.z _returnvalue_2)) false "None"))
    (:`CastFailed`
      (cast `/Game/UE4_Pong/Blueprints/BP_Boundery_Blueprint` OtherActor
        (:`then`
          (`KismetSystemLibrary.PrintString` "Hit" true true (struct :`G` 1.0 :`B` 0.061501 :`A` 1.0))
          (bind _returnvalue_3 (`PrimitiveComponent.GetPhysicsLinearVelocity` _staticmeshcomponent "None"))
          (`PrimitiveComponent.SetPhysicsLinearVelocity` _staticmeshcomponent (`KismetMathLibrary.MakeVector` (* (.x _returnvalue_3) -1.0) (.y _returnvalue_3) (.z _returnvalue_3)) false "None"))
        (:`CastFailed`
          (bind _asbp_paddle_ai (cast `/Game/UE4_Pong/Blueprints/BP_Paddle_AI` OtherActor)
            (:`then`
              (bind _returnvalue_4 (`PrimitiveComponent.GetPhysicsLinearVelocity` (`/Game/UE4_Pong/Blueprints/BP_Paddle_AI.SM_Paddle` _asbp_paddle_ai) "None"))
              (`KismetSystemLibrary.PrintString` "Hit" true true (struct :`G` 1.0 :`B` 0.061501 :`A` 1.0))
              (bind _returnvalue_5 (`PrimitiveComponent.GetPhysicsLinearVelocity` _staticmeshcomponent_2 "None"))
              (`PrimitiveComponent.SetPhysicsLinearVelocity` _staticmeshcomponent_2 (`KismetMathLibrary.MakeVector` (.x _returnvalue_4) (* (.y _returnvalue_5) -1.0) (.z _returnvalue_5)) false "None"))
            (:`CastFailed`
              (cast `/Game/UE4_Pong/Blueprints/BP_GoalLeft` OtherActor
                (:`then`
                  (bind _output_get (set `self.ScoreCPU` (+ (`self.ScoreCPU`) 1)))
                  (`KismetSystemLibrary.PrintString` (`KismetStringLibrary.Conv_IntToString` _output_get) true true (struct :`R` 1.0 :`B` 0.020756 :`A` 1.0))
                  (`KismetSystemLibrary.Delay` 0.5))
                (:`CastFailed`
                  (cast `/Game/UE4_Pong/Blueprints/BP_GoalRight` OtherActor)
                  (bind _output_get_2 (set `self.ScorePlayer` (+ (`self.ScorePlayer`) 1)))
                  (`KismetSystemLibrary.PrintString` (`KismetStringLibrary.Conv_IntToString` _output_get_2) true true (struct :`G` 0.018288 :`B` 1.0 :`A` 1.0))
                  (`KismetSystemLibrary.Delay` 0.5)))
              (bind _outactors (`GameplayStatics.GetAllActorsOfClass` "/Game/UE4_Pong/Blueprints/BP_Paddle_p1.BP_Paddle_p1_C"))
              (for _array_element _outactors
                (`|ExecutionSequence`
                  (:`then_0`
                    (`TextRenderComponent.K2_SetText` (`/Game/UE4_Pong/Blueprints/BP_Paddle_p1.Score_CPU` _array_element) (`KismetTextLibrary.Conv_IntToText` (`self.ScoreCPU`)))
                    (`self.K2_SetActorLocation` (0.0 0.0 0.0))
                    (`PrimitiveComponent.SetPhysicsLinearVelocity` (`self.StaticMeshComponent`) (0.0 1000.0 0.0) false "None")
                    (if (> (`self.ScoreCPU`) 2)
                      (`KismetSystemLibrary.Delay` 1.0)
                      (`KismetSystemLibrary.QuitGame` null "Quit")))
                  (:`then_1`
                    (`TextRenderComponent.K2_SetText` (`/Game/UE4_Pong/Blueprints/BP_Paddle_p1.Score_P1` _array_element) (`KismetTextLibrary.Conv_IntToText` (`self.ScorePlayer`)))
                    (`self.K2_SetActorLocation` (0.0 0.0 0.0))
                    (`PrimitiveComponent.SetPhysicsLinearVelocity` (`self.StaticMeshComponent`) (0.0 -1000.0 0.0) false "None")
                    (if (> (`self.ScorePlayer`) 2)
                      (`KismetSystemLibrary.Delay` 1.0)
                      (`KismetSystemLibrary.QuitGame` null "Quit"))))))))))))

(fn `UserConstructionScript`)